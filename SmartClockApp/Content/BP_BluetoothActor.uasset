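; BP_BluetoothActor sets up the smart clock UI and its Bluetooth link when play begins.
; It creates the BP_Smart_Clock_Main widget with a reference to itself, adds it to the viewport at a fixed size, then requests permissions and reconnects Bluetooth.
; An immediate connection check sets the widget's status text and calls TempDisplay only if connected.
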(event EventBeginPlay
  (bind _returnvalue (Game|GetPlayerController 0))
  (Input|EnableInput _returnvalue)
  (bind _returnvalue_2 (UserInterface|CreateWidget "/Game/BP_Smart_Clock_Main.BP_Smart_Clock_Main_C" _returnvalue "" "" self))
  (Class|UserWidget|SetDesiredSizeinViewport _returnvalue_2 "(X=750.000000,Y=1624.000000)")
  (UserInterface|Viewport|AddtoViewport _returnvalue_2 1)
  (Class|BluetoothManager|RequestPermissions)
  (Class|BluetoothManager|ReconnectBluetooth)
  (bind _returnvalue_3 (Class|BluetoothManager|IsBluetoothConnected))
  (if _returnvalue_3
    (Variables|/Game/BP_Smart_Clock_Main.BP_Smart_Clock_Main_C|SetisConnected _returnvalue_2 "Connected")
    (Default|TempDisplay _returnvalue_2)
    (else
      (Variables|/Game/BP_Smart_Clock_Main.BP_Smart_Clock_Main_C|SetisConnected _returnvalue_2 "Disconnected"))))

(fn ConstructionScript)